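; Guardian weapon attack actor that knocks back any BP_Monster overlapping its GuardianCollision component.
; The push direction runs horizontally from the player character to the monster, setting an end point a short fixed distance beyond it.
; The Moved timeline lerps the monster there, with a separate Z track for a slight vertical offset.
; A single stored target and timeline are shared, so each new overlap replaces the monster being moved.
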(event OnComponentBeginOverlap(GuardianCollision)
  (params (OverlappedComponent :type Primitive%20Component%20Object%20Reference) (OtherActor :type Actor%20Object%20Reference) (OtherComp :type Primitive%20Component%20Object%20Reference) (OtherBodyIndex :type Integer) (bFromSweep :type Boolean) (SweepResult :type Hit%20Result%20Structure%20%28by%20ref%29))
  (bind _asbp_monster (Utilities|Casting|CastToBP_Monster OtherActor))
  (Variables|Default|SetOther%20Actor _asbp_monster)
  (bind _asbp_my_character (Utilities|Casting|CastTobp_myCharacter (Game|Player|GetPlayerPawn 0)))
  (Variables|Default|SetcharacterLocation (Transformation|GetActorLocation _asbp_my_character))
  (Variables|Default|SettargetLocation (Transformation|GetActorLocation (Variables|Default|GetOther%20Actor)))
  (bind _output_get (Variables|Default|Setdirection (- (Math|Vector|MakeVector (.x (Variables|Default|GettargetLocation)) (.y (Variables|Default|GettargetLocation)) (.z (Variables|Default|GettargetLocation))) (Math|Vector|MakeVector (.x (Variables|Default|GetcharacterLocation)) (.y (Variables|Default|GetcharacterLocation)) (.z (Variables|Default|GettargetLocation))))))
  (Variables|Default|SetendLocation (+ (* (Math|Vector|Normalize _output_get) "50.000000,50.000000,0.000000") (Variables|Default|GettargetLocation)))
  (bind (_direction _x__y _z) (Timeline|moved PlayFromStart)
    (:Update
      (Utilities|IsValid (Variables|Default|GetOther%20Actor)
        (:Is%20Valid
          (Transformation|SetActorLocation (Variables|Default|GetOther%20Actor) (Math|Vector|MakeVector (Math|Float|Lerp (.x (Variables|Default|GettargetLocation)) (.x (Variables|Default|GetendLocation)) _x__y) (Math|Float|Lerp (.y (Variables|Default|GettargetLocation)) (.y (Variables|Default|GetendLocation)) _x__y) (Math|Float|Lerp (.z (Variables|Default|GettargetLocation)) (+ (.z (Variables|Default|GettargetLocation)) 1e+01) _z)) false false))))))

(event EventBeginPlay)

(event Collision|EventActorBeginOverlap
  (params (OtherActor :type Actor%20Object%20Reference)))

(event EventTick
  (params (DeltaSeconds :type Float%20%28single-precision%29)))

(fn ConstructionScript)