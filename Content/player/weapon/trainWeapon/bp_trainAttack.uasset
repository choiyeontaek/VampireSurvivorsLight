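; Train attack actor for the player's train weapon that launches whatever actor overlaps its TrainCollision.
; On overlap, a Timeline restarts and teleports that actor each update from StartLocation toward EndLocation.
; Separate XY and Z tracks drive the lerps, with Z blending toward StartLocation plus Height.
; The overlap has no filter, and the graph never sets StartLocation, EndLocation or Height.
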(event OnComponentBeginOverlap(TrainCollision)
  (params (OverlappedComponent :type Primitive%20Component%20Object%20Reference) (OtherActor :type Actor%20Object%20Reference) (OtherComp :type Primitive%20Component%20Object%20Reference) (OtherBodyIndex :type Integer) (bFromSweep :type Boolean) (SweepResult :type Hit%20Result%20Structure%20%28by%20ref%29))
  (bind _startlocation (Variables|Default|GetStartLocation))
  (bind _endlocation (Variables|Default|GetEndLocation))
  (bind (_x _y) (Math|Vector|BreakVector _endlocation))
  (bind (_x_2 _y_2 _z) (Math|Vector|BreakVector _startlocation))
  (bind (_direction _x__y _z_2) (Timeline|Timeline PlayFromStart)
    (:Update
      (Transformation|SetActorLocation OtherActor (Math|Vector|MakeVector (Math|Float|Lerp _x_2 _x _x__y) (Math|Float|Lerp _y_2 _y _x__y) (Math|Float|Lerp _z (+ _z (Variables|Default|GetHeight)) _z_2)) false true))))

(event EventBeginPlay)

(event Collision|EventActorBeginOverlap
  (params (OtherActor :type Actor%20Object%20Reference)))

(event EventTick
  (params (DeltaSeconds :type Float%20%28single-precision%29)))

(fn ConstructionScript)