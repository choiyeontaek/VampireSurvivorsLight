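; BP_LongMonster_Spawner periodically spawns AI-controlled BP_LongMonster pawns in the level.
; BeginPlay starts a looping timer at SpawnInterval that calls LongSpawnActor by name, and prints a debug string.
; Each call gathers every TargetPoint in the level and spawns the monster running BT_LongMonster.
; Location and rotation use separate random picks, so they can come from different target points.
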(event Custom|LongSpawnActor
  (bind _outactors (Actor|GetAllActorsOfClass "/Script/Engine.TargetPoint"))
  (AI|SpawnAIFromClass "/Game/CYT_monster/LongRangeAttack_Monster/BP_LongMonster.BP_LongMonster_C" "/Game/CYT_monster/LongRangeAttack_Monster/BT_LongMonster.BT_LongMonster" (.location (Transformation|GetActorTransform (Utilities|Array|Get(acopy) _outactors (Math|Random|RandomIntegerinRange 0 (- (Utilities|Array|Length _outactors) 1))))) (.rotation (Transformation|GetActorTransform (Utilities|Array|Get(acopy) _outactors (Math|Random|RandomIntegerinRange 0 (- (Utilities|Array|Length _outactors) 1))))) false 0))

(event EventBeginPlay
  (Utilities|Time|SetTimerbyFunctionName 0 "LongSpawnActor" (Variables|Default|GetSpawnInterval) true)
  (Development|PrintString "qoqoqoqoqoqoqooqoqwooqwpe"))

(fn ConstructionScript)