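; Boss enemy that turns toward the player while not attacking, deals contact damage and offers three montage-driven attack events.
; Attacks spawn a radius then a damage plane, start a looping timer dropping swords near the player, or spawn a radius damage actor.
; AnyDamage runs effects for recognized auto-attack and skill damage types, then updates health and both boss widgets.
; Death spawns Experience, shows the end widget and destroys the boss.
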(event OnComponentBeginOverlap(CapsuleComponent)
  (params (OverlappedComponent :type Primitive%20Component%20Object%20Reference) (OtherActor :type Actor%20Object%20Reference) (OtherComp :type Primitive%20Component%20Object%20Reference) (OtherBodyIndex :type Integer) (bFromSweep :type Boolean) (SweepResult :type Hit%20Result%20Structure%20%28by%20ref%29))
  (bind _asmy_character (Utilities|Casting|CastToMyCharacter OtherActor))
  (Game|Damage|ApplyDamage _asmy_character 7.0 0 self "/Game/CYT_monster/Boss/Boss_Tasks/BP_DamageType_BossAttack.BP_DamageType_BossAttack_C"))

(event Custom|Attack
  ;[0.15 0.15 0.15 0.5] 1번 공격  검기
  (Game|SpawnActorfromClass "/Game/CYT_monster/Boss/Skills/Damage/BP_Radius.BP_Radius_C" (Math|Transform|MakeTransform (Transformation|GetWorldLocation (Variables|Default|GetskillOneArrow)) "0, 0, 0" "1.000000,1.000000,1.000000") "Undefined" "MultiplyWithRoot" 0 0) ; 아이템 생성 시키기
  (Utilities|FlowControl|Delay 2.5)
  (Animation|Montage|PlayMontage (Variables|Character|GetMesh) "/Game/CYT_monster/Boss/Animation/aatrox_sheath_to_attack_anm_Montage.aatrox_sheath_to_attack_anm_Montage" 1.0 0.0 "Default"
    (:then
      (Utilities|FlowControl|Delay 0.6)
      (Game|SpawnActorfromClass "/Game/CYT_monster/Boss/Skills/Damage/BP_DamagePlane.BP_DamagePlane_C" (Math|Transform|MakeTransform (Transformation|GetWorldLocation (Variables|Default|GetskillOneArrow)) "0, 0, 0" "1.000000,1.000000,1.000000") "Undefined" "MultiplyWithRoot" 0 0) ; 아이템 생성 시키기
    )))

(event Custom|AttackSword
  ;[0.15 0.15 0.15 0.5] 2번 공격  소드
  (Animation|Montage|PlayMontage (Variables|Character|GetMesh) "/Game/CYT_monster/Boss/Animation/aatrox_passive_attack_anm_Montage.aatrox_passive_attack_anm_Montage" 1.0 0.0 "Default"
    (:then
      (Utilities|Time|SetTimerbyFunctionName 0 "Sword" 1.0 true))))

(event Custom|AttackSkill
  ;[0.15 0.15 0.15 0.5] 3번 공격 내려찍기
  (Utilities|FlowControl|Delay 0.2)
  (Animation|Montage|PlayMontage (Variables|Character|GetMesh) "/Game/CYT_monster/Boss/Animation/aatrox_crit_anm_Montage.aatrox_crit_anm_Montage"
    (:then
      (Utilities|FlowControl|Delay 0.4)
      (Game|SpawnActorfromClass "/Game/CYT_monster/Boss/Skills/Damage/BP_RadiusDamage.BP_RadiusDamage_C" (Math|Transform|MakeTransform (Transformation|GetWorldLocation (Variables|Default|GetskillOneArrow)) "0, 0, 0" "1.000000,1.000000,1.000000") "Undefined" "MultiplyWithRoot" 0 0) ; 아이템 생성 시키기
    )))

(event Custom|Sword
  (bind _returnvalue (Game|GetPlayerCharacter 0))
  (bind _returnvalue_2 (Transformation|GetActorLocation _returnvalue))
  ;[0.15 0.15 0.15 0.5] 2번 공격  소드
  (Game|SpawnActorfromClass "/Game/CYT_monster/Boss/Skills/Sword/BP_Sword.BP_Sword_C" (Math|Transform|MakeTransform (Math|Vector|MakeVector (Math|Random|RandomFloatinRange (- (.x _returnvalue_2) 2e+03) (+ (.x _returnvalue_2) 2e+03)) (+ (.y _returnvalue_2) 2e+03) (.z _returnvalue_2)) "0.000000,-90.000000,0.000000" "1.000000,1.000000,1.000000") "Undefined" "MultiplyWithRoot" 0 0))

(event EventTick
  (params (DeltaSeconds :type Float%20%28single-precision%29))
  ;[0.15 0.15 0.15 0.5] 플레이어 이동 방향 으로 회전 시키는방법
  (if (not (Variables|Default|GetAttacking?))
    (Transformation|SetActorRotation (Math|Rotator|MakeRotator 0.0 0.0 (.yaw (Math|Rotator|FindLookatRotation (Transformation|GetActorLocation) (Transformation|GetActorLocation (Game|Player|GetPlayerPawn 0))))))))

(event Game|Damage|EventAnyDamage
  (params (Damage :type Float%20%28single-precision%29) (DamageType :type Damage%20Type%20Object%20Reference) (InstigatedBy :type Controller%20Object%20Reference) (DamageCauser :type Actor%20Object%20Reference))
  ;[0.15 0.15 0.15 0.5] 데미지 받기 타입정리
  (Variables|Default|SetDamage Damage)
  (Variables|Default|SetDamage%20Type DamageType)
  (Variables|Default|SetDamage%20Causer DamageCauser)
  (Variables|Default|SetInstigated%20By InstigatedBy)
  (Utilities|FlowControl|Sequence
    (:then_0
      (if (Class|GameplayStatics|ObjectIsA (Variables|Default|GetDamage%20Type) "/Script/VamSurLight.AutoAttackDamageType")
        (bind _asauto_attack_damage_type (Utilities|Casting|CastToAutoAttackDamageType (Variables|Default|GetDamage%20Type)))
        (Class|BaseDamageType|ApplyDamageEffectImplementation _asauto_attack_damage_type self (Variables|Default|GetDamage) (Variables|Default|GetInstigated%20By) (Variables|Default|GetDamage%20Causer))
        (bind _output_get (Variables|Default|SetCurrentHealth (- (Variables|Default|GetCurrentHealth) (Variables|Default|GetDamage)) :!label _label))
        (Default|BossUpdate (Variables|Default|GetHealthUI) _output_get (Variables|Default|GetMaxHealth))
        (Default|BossUpdate (Variables|Default|GetBossHaelth) _output_get (Variables|Default|GetMaxHealth))
        (if (<= _output_get 0.0)
          (Game|SpawnActorfromClass "/Script/VamSurLight.Experience" (Math|Transform|MakeTransform (Transformation|GetActorLocation) (Transformation|GetActorRotation) "1.000000,1.000000,1.000000") "Undefined" "MultiplyWithRoot" 0 0) ; 아이템 생성 시키기
          (bind _returnvalue (UserInterface|CreateWidget "/Game/GameWidget/widget_End.widget_End_C"))
          (UserInterface|Viewport|AddtoViewport _returnvalue 0)
          (Actor|DestroyActor))))
    (:then_1
      (if (Class|GameplayStatics|ObjectIsA (Variables|Default|GetDamage%20Type) "/Script/VamSurLight.SkillBoomerangDamageType")
        (bind _asskill_boomerang_damage_type (Utilities|Casting|CastToSkillBoomerangDamageType (Variables|Default|GetDamage%20Type)))
        (Class|BaseDamageType|ApplyDamageEffectImplementation _asskill_boomerang_damage_type self (Variables|Default|GetDamage) (Variables|Default|GetInstigated%20By) (Variables|Default|GetDamage%20Causer))
        (goto _label)))
    (:then_2
      (if (Class|GameplayStatics|ObjectIsA (Variables|Default|GetDamage%20Type) "/Script/VamSurLight.SkillForceFieldDamageType")
        (bind _asskill_force_field_damage_type (Utilities|Casting|CastToSkillForceFieldDamageType (Variables|Default|GetDamage%20Type)))
        (Class|BaseDamageType|ApplyDamageEffectImplementation _asskill_force_field_damage_type self (Variables|Default|GetDamage) (Variables|Default|GetInstigated%20By) (Variables|Default|GetDamage%20Causer))
        (goto _label)))
    (:then_3
      (if (Class|GameplayStatics|ObjectIsA (Variables|Default|GetDamage%20Type) "/Script/VamSurLight.SkillGuardianDamageType")
        (bind _asskill_guardian_damage_type (Utilities|Casting|CastToSkillGuardianDamageType (Variables|Default|GetDamage%20Type)))
        (Class|BaseDamageType|ApplyDamageEffectImplementation _asskill_guardian_damage_type self (Variables|Default|GetDamage) (Variables|Default|GetInstigated%20By) (Variables|Default|GetDamage%20Causer))
        (goto _label)))
    (:then_4
      (if (Class|GameplayStatics|ObjectIsA (Variables|Default|GetDamage%20Type) "/Script/VamSurLight.SkillTrainDamageType")
        (bind _asskill_train_damage_type (Utilities|Casting|CastToSkillTrainDamageType (Variables|Default|GetDamage%20Type)))
        (Class|BaseDamageType|ApplyDamageEffectImplementation _asskill_train_damage_type self (Variables|Default|GetDamage) (Variables|Default|GetInstigated%20By) (Variables|Default|GetDamage%20Causer))
        (goto _label)))))

(event EventBeginPlay
  (Utilities|FlowControl|Sequence
    (:then_0
      (bind _returnvalue (UserInterface|CreateWidget "/Game/CYT_monster/Boss/WB_Screen.WB_Screen_C"))
      (bind _output_get (Variables|Default|SetHealthUI _returnvalue))
      (UserInterface|Viewport|AddtoViewport _output_get 0)
      (bind _output_get_2 (Variables|Default|SetCurrentHealth (Variables|Default|GetMaxHealth)))
      (Default|BossUpdate (Variables|Default|GetHealthUI) _output_get_2 (Variables|Default|GetMaxHealth)))
    (:then_1
      (bind _returnvalue_2 (UserInterface|CreateWidget "/Game/CYT_monster/Boss/WB_Boss.WB_Boss_C"))
      (bind _output_get_3 (Variables|Default|SetBossHaelth _returnvalue_2))
      (Variables|Default|SetWB_Boss 0)
      (bind _output_get_4 (Variables|Default|SetCurrentHealth (Variables|Default|GetMaxHealth)))
      (Default|BossUpdate _output_get_3 _output_get_4 (Variables|Default|GetMaxHealth)))))

(fn ConstructionScript)