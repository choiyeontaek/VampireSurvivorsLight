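; Long-range monster enemy that turns to face the player every tick and damages the player character on capsule overlap.
; FireProjectile spawns a bullet at FirePoint and plays a montage; nothing live in this file calls it.
; AnyDamage spawns a damage actor and sound, then matches auto-attack or skill damage types for effects and health loss.
; At zero health it drops Experience and destroys itself.
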(event OnComponentHit(CapsuleComponent)
  (params (HitComponent :type Primitive%20Component%20Object%20Reference) (OtherActor :type Actor%20Object%20Reference) (OtherComp :type Primitive%20Component%20Object%20Reference) (NormalImpulse :type Vector :default "0, 0, 0") (Hit :type Hit%20Result%20Structure%20%28by%20ref%29))
  ;[0.15 0.15 0.15 0.5] Comment
)

(event OnComponentBeginOverlap(CapsuleComponent)
  (params (OverlappedComponent :type Primitive%20Component%20Object%20Reference) (OtherActor :type Actor%20Object%20Reference) (OtherComp :type Primitive%20Component%20Object%20Reference) (OtherBodyIndex :type Integer) (bFromSweep :type Boolean) (SweepResult :type Hit%20Result%20Structure%20%28by%20ref%29))
  (bind _asmy_character (Utilities|Casting|CastToMyCharacter OtherActor))
  (Game|Damage|ApplyDamage _asmy_character 7.0 0 self "/Game/CYT_monster/LongRangeAttack_Monster/L_Tasks/BP_DamageType_LongRangeAttackangeAttack.BP_DamageType_LongRangeAttackangeAttack_C"))

(event Custom|FireProjectile
  ;[0.15 0.15 0.15 0.5] 월드에서 에로우포인터컴포넌트에   구체 생성
  (Game|SpawnActorfromClass "/Game/CYT_monster/LongRangeAttack_Monster/VFX/BP_Bullet.BP_Bullet_C" (Transformation|GetWorldTransform (Variables|Default|GetFirePoint)) "Undefined" "MultiplyWithRoot" 0 0)
  (Animation|Montage|PlayMontage (Variables|Character|GetMesh) "/Game/CYT_monster/LongRangeAttack_Monster/LongAnimation/chaman-ti-pche-3-animations/source/Anim_1_Ti-Pche_Rig_Montage.Anim_1_Ti-Pche_Rig_Montage" 1.0 0.0 "Default"))

(event Collision|EventActorBeginOverlap
  (params (OtherActor :type Actor%20Object%20Reference)))

(event EventBeginPlay
  (Variables|Default|SetCurrentHealth (Variables|Default|GetMaxHealth)))

(event EventTick
  (params (DeltaSeconds :type Float%20%28single-precision%29))
  ;[0.15 0.15 0.15 0.5] 플레이어 이동 방향 으로 회전 시키는방법
  (Transformation|SetActorRotation (Math|Rotator|MakeRotator 0.0 0.0 (.yaw (Math|Rotator|FindLookatRotation (Transformation|GetActorLocation) (Transformation|GetActorLocation (Game|Player|GetPlayerPawn 0)))))))

(event Game|Damage|EventAnyDamage
  (params (Damage :type Float%20%28single-precision%29) (DamageType :type Damage%20Type%20Object%20Reference) (InstigatedBy :type Controller%20Object%20Reference) (DamageCauser :type Actor%20Object%20Reference))
  (bind _returnvalue (Transformation|GetActorLocation))
  (Game|SpawnActorfromClass "/Game/player/widget/damage/bp_damage.bp_damage_C" (Transformation|GetActorTransform) "Undefined" "MultiplyWithRoot" 0 (Math|Float|Truncate Damage) 0)
  (Variables|Default|SetDamage Damage)
  (Variables|Default|SetDamage%20Type DamageType)
  (Variables|Default|SetDamage%20Causer DamageCauser)
  (Variables|Default|SetInstigated%20By InstigatedBy)
  (Utilities|FlowControl|Sequence
    (:then_0
      (if (Class|GameplayStatics|ObjectIsA (Variables|Default|GetDamage%20Type) "/Script/VamSurLight.AutoAttackDamageType")
        (bind _asauto_attack_damage_type (Utilities|Casting|CastToAutoAttackDamageType (Variables|Default|GetDamage%20Type)))
        (Class|BaseDamageType|ApplyDamageEffectImplementation _asauto_attack_damage_type self (Variables|Default|GetDamage) (Variables|Default|GetInstigated%20By) (Variables|Default|GetDamage%20Causer))
        (Niagara|SpawnSystematLocation "/Game/MixedVFX/Particles/Projectiles/Hits/NS_FairyArrow_Hit.NS_FairyArrow_Hit" _returnvalue "0, 0, 0" "2.000000,2.000000,2.000000")
        (bind _output_get (Variables|Default|SetCurrentHealth (- (Variables|Default|GetCurrentHealth) (Variables|Default|GetDamage)) :!label _label))
        (if (<= _output_get 0.0)
          (Game|SpawnActorfromClass "/Script/VamSurLight.Experience" (Math|Transform|MakeTransform (Transformation|GetActorLocation) (Transformation|GetActorRotation) "1.000000,1.000000,1.000000") "Undefined" "MultiplyWithRoot" 0 0) ; 아이템 생성 시키기
          (Actor|DestroyActor))))
    (:then_1
      (if (Class|GameplayStatics|ObjectIsA (Variables|Default|GetDamage%20Type) "/Script/VamSurLight.SkillBoomerangDamageType")
        (bind _asskill_boomerang_damage_type (Utilities|Casting|CastToSkillBoomerangDamageType (Variables|Default|GetDamage%20Type)))
        (Class|BaseDamageType|ApplyDamageEffectImplementation _asskill_boomerang_damage_type self (Variables|Default|GetDamage) (Variables|Default|GetInstigated%20By) (Variables|Default|GetDamage%20Causer))
        (Niagara|SpawnSystematLocation "/Game/MixedVFX/Particles/Projectiles/Hits/NS_Shuriken_04_Hit.NS_Shuriken_04_Hit" _returnvalue "0, 0, 0" "2.000000,2.000000,2.000000")
        (goto _label)))
    (:then_2
      (if (Class|GameplayStatics|ObjectIsA (Variables|Default|GetDamage%20Type) "/Script/VamSurLight.SkillForceFieldDamageType")
        (bind _asskill_force_field_damage_type (Utilities|Casting|CastToSkillForceFieldDamageType (Variables|Default|GetDamage%20Type)))
        (Class|BaseDamageType|ApplyDamageEffectImplementation _asskill_force_field_damage_type self (Variables|Default|GetDamage) (Variables|Default|GetInstigated%20By) (Variables|Default|GetDamage%20Causer))
        (Niagara|SpawnSystematLocation "/Game/MixedVFX/Particles/Projectiles/Hits/NS_HolyArrow_Hit.NS_HolyArrow_Hit" _returnvalue "0, 0, 0" "2.000000,2.000000,2.000000")
        (goto _label)))
    (:then_3
      (if (Class|GameplayStatics|ObjectIsA (Variables|Default|GetDamage%20Type) "/Script/VamSurLight.SkillGuardianDamageType")
        (bind _asskill_guardian_damage_type (Utilities|Casting|CastToSkillGuardianDamageType (Variables|Default|GetDamage%20Type)))
        (Class|BaseDamageType|ApplyDamageEffectImplementation _asskill_guardian_damage_type self (Variables|Default|GetDamage) (Variables|Default|GetInstigated%20By) (Variables|Default|GetDamage%20Causer))
        (Niagara|SpawnSystematLocation "/Game/MixedVFX/Particles/Projectiles/Hits/NS_Shuriken_03_Hit.NS_Shuriken_03_Hit" _returnvalue "0, 0, 0" "2.000000,2.000000,2.000000")
        (goto _label)))
    (:then_4
      (if (Class|GameplayStatics|ObjectIsA (Variables|Default|GetDamage%20Type) "/Script/VamSurLight.SkillTrainDamageType")
        (bind _asskill_train_damage_type (Utilities|Casting|CastToSkillTrainDamageType (Variables|Default|GetDamage%20Type)))
        (Class|BaseDamageType|ApplyDamageEffectImplementation _asskill_train_damage_type self (Variables|Default|GetDamage) (Variables|Default|GetInstigated%20By) (Variables|Default|GetDamage%20Causer))
        (Niagara|SpawnSystematLocation "/Game/MixedVFX/Particles/Projectiles/Hits/NS_LightningBolt_Hit.NS_LightningBolt_Hit" _returnvalue "0, 0, 0" "2.000000,2.000000,2.000000")
        (goto _label)))
    (:then_5
      (Audio|PlaySound2D "/Game/sound/get_damage_Cue.get_damage_Cue" 0.1 1.0 0.0 0 0))))

(fn ConstructionScript)