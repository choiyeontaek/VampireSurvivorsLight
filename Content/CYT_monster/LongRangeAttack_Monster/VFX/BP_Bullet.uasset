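; Projectile for the long-range attack monster that damages the player character on contact.
; A sphere overlap applies fixed damage to MyCharacter with the long-skill damage type, without destroying the bullet, which removes itself after a timed lifespan.
; When the bullet itself takes auto-attack damage, it hands the hit to that damage type's effect implementation with itself as target.
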(event OnComponentBeginOverlap(Sphere)
  (params (OverlappedComponent :type Primitive%20Component%20Object%20Reference) (OtherActor :type Actor%20Object%20Reference) (OtherComp :type Primitive%20Component%20Object%20Reference) (OtherBodyIndex :type Integer) (bFromSweep :type Boolean) (SweepResult :type Hit%20Result%20Structure%20%28by%20ref%29))
  (bind _asmy_character (Utilities|Casting|CastToMyCharacter OtherActor))
  (Game|Damage|ApplyDamage _asmy_character 7.0 0 self "/Game/CYT_monster/LongRangeAttack_Monster/L_Tasks/BP_DamageType_LongSkill.BP_DamageType_LongSkill_C"))

(event EventBeginPlay
  (Utilities|FlowControl|Delay 8.0)
  (Actor|DestroyActor))

(event Game|Damage|EventAnyDamage
  (params (Damage :type Float%20%28single-precision%29) (DamageType :type Damage%20Type%20Object%20Reference) (InstigatedBy :type Controller%20Object%20Reference) (DamageCauser :type Actor%20Object%20Reference))
  (if (Class|GameplayStatics|ObjectIsA DamageType "/Script/VamSurLight.AutoAttackDamageType")
    (bind _asauto_attack_damage_type (Utilities|Casting|CastToAutoAttackDamageType DamageType))
    (Class|BaseDamageType|ApplyDamageEffectImplementation _asauto_attack_damage_type self Damage 0 DamageCauser)))

(fn ConstructionScript)