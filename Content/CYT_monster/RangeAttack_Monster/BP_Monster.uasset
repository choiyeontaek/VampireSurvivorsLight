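; Enemy monster from the RangeAttack_Monster set that turns to face the player every tick and deals range-attack typed damage to the player on capsule overlap.
; AnyDamage branches on player attack and skill damage types, runs each type's effect, then subtracts health, spawning Experience and destroying itself at zero.
; Boomerang and Train hits also launch it through a Timeline-lerped displacement with a height curve, which ignores the passed Time.
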(event OnComponentBeginOverlap(CapsuleComponent)
  (params (OverlappedComponent :type Primitive%20Component%20Object%20Reference) (OtherActor :type Actor%20Object%20Reference) (OtherComp :type Primitive%20Component%20Object%20Reference) (OtherBodyIndex :type Integer) (bFromSweep :type Boolean) (SweepResult :type Hit%20Result%20Structure%20%28by%20ref%29))
  (bind _asmy_character (Utilities|Casting|CastToMyCharacter OtherActor))
  (Game|Damage|ApplyDamage _asmy_character 7.0 0 self "/Game/CYT_monster/RangeAttack_Monster/S_Tasks/BP_DamageType_RangeAttack.BP_DamageType_RangeAttack_C"))

(event Custom|EventTrain
  (params (StartLocation :type Vector) (EndLocation :type Vector) (Height :type Float%20%28double-precision%29) (Time :type Float%20%28double-precision%29))
  (bind _output_get (Variables|Default|SetStart%20Location StartLocation))
  (bind _output_get_2 (Variables|Default|SetEnd%20Location EndLocation))
  (bind (_direction _x__y _z) (Timeline|Train PlayFromStart)
    (:Update
      (Transformation|SetActorLocation (Math|Vector|MakeVector (Math|Float|Lerp (.X (Math|Vector|BreakVector _output_get)) (.X (Math|Vector|BreakVector _output_get_2)) _x__y) (Math|Float|Lerp (.Y (Math|Vector|BreakVector _output_get)) (.Y (Math|Vector|BreakVector _output_get_2)) _x__y) (Math|Float|Lerp (.Z (Math|Vector|BreakVector _output_get)) (+ (.Z (Math|Vector|BreakVector _output_get)) Height) _z)) false false))))

(event EventBeginPlay
  (Variables|Default|SetCurrentHealth (Variables|Default|GetMaxHealth)))

(event EventTick
  (params (DeltaSeconds :type Float%20%28single-precision%29))
  ;[0.15 0.15 0.15 0.5] 플레이어 이동 방향 으로 회전 시키는방법
  (Transformation|SetActorRotation (Math|Rotator|MakeRotator 0.0 0.0 (.yaw (Math|Rotator|FindLookatRotation (Transformation|GetActorLocation) (Transformation|GetActorLocation (Game|Player|GetPlayerPawn 0)))))))

(event Game|Damage|EventAnyDamage
  (params (Damage :type Float%20%28single-precision%29) (DamageType :type Damage%20Type%20Object%20Reference) (InstigatedBy :type Controller%20Object%20Reference) (DamageCauser :type Actor%20Object%20Reference))
  (Variables|Default|SetDamage Damage)
  (Variables|Default|SetDamage%20Type DamageType)
  (Variables|Default|SetDamage%20Causer DamageCauser)
  (Variables|Default|SetInstigated%20By InstigatedBy)
  (Utilities|FlowControl|Sequence
    (:then_0
      (if (Class|GameplayStatics|ObjectIsA (Variables|Default|GetDamage%20Type) "/Script/VamSurLight.AutoAttackDamageType")
        (bind _asauto_attack_damage_type (Utilities|Casting|CastToAutoAttackDamageType (Variables|Default|GetDamage%20Type)))
        (Class|BaseDamageType|ApplyDamageEffectImplementation _asauto_attack_damage_type self (Variables|Default|GetDamage) (Variables|Default|GetInstigated%20By) (Variables|Default|GetDamage%20Causer))
        (bind _output_get (Variables|Default|SetCurrentHealth (- (Variables|Default|GetCurrentHealth) (Variables|Default|GetDamage)) :!label _label))
        (if (<= _output_get 0.0)
          (Game|SpawnActorfromClass "/Script/VamSurLight.Experience" (Math|Transform|MakeTransform (Transformation|GetActorLocation) (Transformation|GetActorRotation) "1.000000,1.000000,1.000000") "Undefined" "MultiplyWithRoot" 0 0) ; 아이템 생성 시키기
          (Actor|DestroyActor))))
    (:then_1
      (if (Class|GameplayStatics|ObjectIsA (Variables|Default|GetDamage%20Type) "/Script/VamSurLight.SkillBoomerangDamageType")
        (bind _asskill_boomerang_damage_type (Utilities|Casting|CastToSkillBoomerangDamageType (Variables|Default|GetDamage%20Type)))
        (Class|BaseDamageType|ApplyDamageEffectImplementation _asskill_boomerang_damage_type self (Variables|Default|GetDamage) (Variables|Default|GetInstigated%20By) (Variables|Default|GetDamage%20Causer))
        (CallFunction|TrainDamage (Variables|/Script/VamSurLight.BaseDamageType|GetStartLocation _asskill_boomerang_damage_type) (Variables|/Script/VamSurLight.BaseDamageType|GetEndLocation _asskill_boomerang_damage_type) (Variables|/Script/VamSurLight.BaseDamageType|GetHeight _asskill_boomerang_damage_type) 2.0)
        (goto _label)))
    (:then_2
      (if (Class|GameplayStatics|ObjectIsA (Variables|Default|GetDamage%20Type) "/Script/VamSurLight.SkillForceFieldDamageType")
        (bind _asskill_force_field_damage_type (Utilities|Casting|CastToSkillForceFieldDamageType (Variables|Default|GetDamage%20Type)))
        (Class|BaseDamageType|ApplyDamageEffectImplementation _asskill_force_field_damage_type self (Variables|Default|GetDamage) (Variables|Default|GetInstigated%20By) (Variables|Default|GetDamage%20Causer))
        (goto _label)))
    (:then_3
      (if (Class|GameplayStatics|ObjectIsA (Variables|Default|GetDamage%20Type) "/Script/VamSurLight.SkillGuardianDamageType")
        (bind _asskill_guardian_damage_type (Utilities|Casting|CastToSkillGuardianDamageType (Variables|Default|GetDamage%20Type)))
        (Class|BaseDamageType|ApplyDamageEffectImplementation _asskill_guardian_damage_type self (Variables|Default|GetDamage) (Variables|Default|GetInstigated%20By) (Variables|Default|GetDamage%20Causer))
        (goto _label)))
    (:then_4
      (if (Class|GameplayStatics|ObjectIsA (Variables|Default|GetDamage%20Type) "/Script/VamSurLight.SkillTrainDamageType")
        (bind _asskill_train_damage_type (Utilities|Casting|CastToSkillTrainDamageType (Variables|Default|GetDamage%20Type)))
        (Class|BaseDamageType|ApplyDamageEffectImplementation _asskill_train_damage_type self (Variables|Default|GetDamage) (Variables|Default|GetInstigated%20By) (Variables|Default|GetDamage%20Causer))
        (CallFunction|TrainDamage (Variables|/Script/VamSurLight.BaseDamageType|GetStartLocation _asskill_train_damage_type) (Variables|/Script/VamSurLight.BaseDamageType|GetEndLocation _asskill_train_damage_type) (Variables|/Script/VamSurLight.BaseDamageType|GetHeight _asskill_train_damage_type) 2.0)
        (goto _label)))))

(fn ConstructionScript)

(fn TrainDamage
  (params (StartLocation :type Vector) (EndLocation :type Vector) (Height :type Float%20%28double-precision%29) (Time :type Float%20%28double-precision%29))
  (CallFunction|EventTrain StartLocation EndLocation Height Time))