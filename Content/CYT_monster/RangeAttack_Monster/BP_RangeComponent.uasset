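; BP_RangeComponent is a component that periodically spawns BP_Monster AI around its owning actor.
; After a short delay on BeginPlay, it starts a looping SpawnRange timer at SpawnInterval0 and prints a debug message.
; Each tick of that timer spawns a monster running BT_Monster at a random reachable navmesh point within a randomized radius of the owner.
; An alternative TargetPoint-based spawn location is left unconnected.
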(event Custom|SpawnRange
  (AI|SpawnAIFromClass "/Game/CYT_monster/RangeAttack_Monster/BP_Monster.BP_Monster_C" "/Game/CYT_monster/RangeAttack_Monster/BT_Monster.BT_Monster" (.RandomLocation (AI|Navigation|GetRandomReachablePointinRadius (Transformation|GetActorLocation (Components|GetOwner)) (Math|Random|RandomFloatinRange 1.5e+03 2.5e+03) 0 0)) "0, 0, 0" false 0))

(event EventBeginPlay
  (Utilities|FlowControl|Delay 2.0)
  (Utilities|Time|SetTimerbyFunctionName 0 "SpawnRange" (Variables|Default|GetSpawnInterval_0) true)
  (Development|PrintString "Hello"))

(event EventTick
  (params (DeltaSeconds :type Float%20%28single-precision%29)))